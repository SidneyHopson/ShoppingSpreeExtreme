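; Shopping cart actor that collects items from the player's shopping list and triggers the win at checkout.
; When a Cube_Blueprint overlaps its box, Attach decrements the matching Player item quantity, clears both hands, disables physics and collision, and snaps it to the next of fifteen mesh sockets.
; Overlapping a CashierBox calls Player.Win if all five quantities are zero; an unused branch recounts cart contents instead.
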(event `self.ReceiveBeginPlay`
  (bind _asplayer (cast `/Game/Blueprints/Player` (`GameplayStatics.GetPlayerCharacter` 0)))
  (set `self.Player` _asplayer))

(event `self.Box.OnComponentBeginOverlap`
  (params (OverlappedComponent :type "PrimitiveComponent Object Reference") (OtherActor :type "Actor Object Reference") (OtherComp :type "PrimitiveComponent Object Reference") (OtherBodyIndex :type Integer) (bFromSweep :type Boolean) (SweepResult :type "HitResult Structure (by ref)"))
  (bind _ascube_blueprint (cast `/Game/Blueprints/Items/Cube_Blueprint` OtherActor))
  (`self.Attach` _ascube_blueprint))

(event `self.ReceiveActorBeginOverlap`
  (params (OtherActor :type "Actor Object Reference"))
  (cast `/Game/Blueprints/CashierBox` OtherActor)
  (`self.CheckIfDone`))

(fn `Attach`
  (params (`Object to attach` :type "/Game/Blueprints/Items/Cube_Blueprint Object Reference"))
  (bind _returnvalue (`GameplayStatics.GetObjectClass` `Object to attach`))
  (bind _player (`self.Player`))
  (bind _player_2 (`self.Player`))
  (bind _player_3 (`self.Player`))
  (bind _staticmeshcomponent (`StaticMeshActor.StaticMeshComponent` `Object to attach`))
  (if (and (== _returnvalue (`GameplayStatics.GetObjectClass` (`/Game/Blueprints/Player.Item1` _player))) (!= (`/Game/Blueprints/Player.Item1Quantity` _player) 0))
    (set `/Game/Blueprints/Player.Item1Quantity` (- (`/Game/Blueprints/Player.Item1Quantity` _player_3) 1) _player_3)
    (`self.K2_DetachFromActor` `Object to attach` "KeepWorld" "KeepWorld" "KeepWorld" :!label _label)
    (set `/Game/Blueprints/Player.CurrentLeftHandItem` null _player_2)
    (set `/Game/Blueprints/Player.CurrentRightHandItem` null _player_2)
    (`PrimitiveComponent.SetSimulatePhysics` _staticmeshcomponent false)
    (`PrimitiveComponent.SetCollisionEnabled` _staticmeshcomponent "NoCollision")
    (`self.K2_AttachToComponent` `Object to attach` (`self.StaticMesh`) (`self.NextAvailableSocket`) "SnapToTarget" "SnapToTarget" "KeepRelative" true)
    (set `/Game/Blueprints/Items/Cube_Blueprint.Spawning` true `Object to attach`)
    (`KismetArrayLibrary.Array_Add` (`self.ItemsInCart`) `Object to attach`)
    (`self.Set Next Socket`)
    (elif (and (== _returnvalue (`GameplayStatics.GetObjectClass` (`/Game/Blueprints/Player.Item2` _player))) (!= (`/Game/Blueprints/Player.Item2Quantity` _player) 0))
      (set `/Game/Blueprints/Player.Item2Quantity` (- (`/Game/Blueprints/Player.Item2Quantity` _player_3) 1) _player_3)
      (goto _label)
      (elif (and (== _returnvalue (`GameplayStatics.GetObjectClass` (`/Game/Blueprints/Player.Item3` _player))) (!= (`/Game/Blueprints/Player.Item3Quantity` _player) 0))
        (set `/Game/Blueprints/Player.Item3Quantity` (- (`/Game/Blueprints/Player.Item3Quantity` _player_3) 1) _player_3)
        (goto _label)
        (elif (and (== _returnvalue (`GameplayStatics.GetObjectClass` (`/Game/Blueprints/Player.Item4` _player))) (!= (`/Game/Blueprints/Player.Item4Quantity` _player) 0))
          (set `/Game/Blueprints/Player.Item4Quantity` (- (`/Game/Blueprints/Player.Item4Quantity` _player_3) 1) _player_3)
          (goto _label)
          (elif (and (== _returnvalue (`GameplayStatics.GetObjectClass` (`/Game/Blueprints/Player.Item5` _player))) (!= (`/Game/Blueprints/Player.Item5Quantity` _player) 0))
            (set `/Game/Blueprints/Player.Item5Quantity` (- (`/Game/Blueprints/Player.Item5Quantity` _player_3) 1) _player_3)
            (goto _label)))))))

(fn `CheckIfDone`
  (locals (Item1Quantity :type Integer) (Item2Quantity :type Integer) (Item3Quantity :type Integer) (Item4Quantity :type Integer) (Item5Quantity :type Integer))
  (bind _player (`self.Player`))
  (if (and (== (`/Game/Blueprints/Player.Item1Quantity` _player) 0) (== (`/Game/Blueprints/Player.Item2Quantity` _player) 0) (== (`/Game/Blueprints/Player.Item3Quantity` _player) 0) (== (`/Game/Blueprints/Player.Item4Quantity` _player) 0) (== (`/Game/Blueprints/Player.Item5Quantity` _player) 0))
    (`/Game/Blueprints/Player.Win` (`self.Player`))))

(fn `Set Next Socket`
  (switch `name` (`self.NextAvailableSocket`)
    (:`Item1`
      (set `self.NextAvailableSocket` "Item2"))
    (:`Item2`
      (set `self.NextAvailableSocket` "Item3"))
    (:`Item3`
      (set `self.NextAvailableSocket` "Item4"))
    (:`Item4`
      (set `self.NextAvailableSocket` "Item5"))
    (:`Item5`
      (set `self.NextAvailableSocket` "Item6"))
    (:`Item6`
      (set `self.NextAvailableSocket` "Item7"))
    (:`Item7`
      (set `self.NextAvailableSocket` "Item8"))
    (:`Item8`
      (set `self.NextAvailableSocket` "Item9"))
    (:`Item9`
      (set `self.NextAvailableSocket` "Item10"))
    (:`Item10`
      (set `self.NextAvailableSocket` "Item11"))
    (:`Item11`
      (set `self.NextAvailableSocket` "Item12"))
    (:`Item12`
      (set `self.NextAvailableSocket` "Item13"))
    (:`Item13`
      (set `self.NextAvailableSocket` "Item14"))
    (:`Item14`
      (set `self.NextAvailableSocket` "Item15"))
    (:`Item15`
      (set `self.Full` true))))

(fn `UserConstructionScript`)