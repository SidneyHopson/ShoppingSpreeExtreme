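; FindPathPoint is an AI behavior tree task that finds the current patrol point for a BP_NPCBase pawn.
; It reads the point at the blackboard path index from the NPC's PatrolPath and transforms it from the path actor's local space to world space.
; It writes the result to the blackboard path vector and finishes successfully.
; A failed cast or invalid path leaves the task without a FinishExecute call.
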(event `self.ReceiveExecuteAI`
  (params (OwnerController :type "AIController Object Reference") (ControlledPawn :type "Pawn Object Reference"))
  (bind _asbp_npcbase (cast `/Game/Blueprints/AI/BP_NPCBase` ControlledPawn))
  (bind _patrolpath (`/Game/Blueprints/AI/BP_NPCBase.PatrolPath` _asbp_npcbase)
    (:`then`
      (`BTFunctionLibrary.SetBlackboardValueAsVector` (`self.BB_PathVector`) (`KismetMathLibrary.TransformLocation` (`Actor.GetTransform` _patrolpath) (`|GetArrayItem` (`/Game/Blueprints/AI/PatrolPath.PathPoint` _patrolpath) (`BTFunctionLibrary.GetBlackboardValueAsInt` (`self.BB_PathIndex`)))))
      (`self.FinishExecute` true))
    (:`else`)))