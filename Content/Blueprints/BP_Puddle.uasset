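; Puddle hazard that makes the player slip when they enter its box trigger.
; On overlap it switches the Player to Flying movement, doubles MaxFlySpeed and plays a slip sound.
; A looping timer calls LeavePuddle, which after a short delay restores Walking on player 0 and clears the timer.
; The fly speed is never restored, so each overlap compounds it.
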(event `self.Box.OnComponentBeginOverlap`
  (params (OverlappedComponent :type "PrimitiveComponent Object Reference") (OtherActor :type "Actor Object Reference") (OtherComp :type "PrimitiveComponent Object Reference") (OtherBodyIndex :type Integer) (bFromSweep :type Boolean) (SweepResult :type "HitResult Structure (by ref)"))
  (bind _asplayer (cast `/Game/Blueprints/Player` OtherActor))
  (bind _charactermovement (`Character.CharacterMovement` _asplayer))
  (`CharacterMovementComponent.SetMovementMode` _charactermovement "MOVE_Flying" 0)
  (bind _returnvalue (`KismetSystemLibrary.K2_SetTimerDelegate` (delegate `LeavePuddle`) 0.5 true))
  (set `CharacterMovementComponent.MaxFlySpeed` (* 2 (`CharacterMovementComponent.MaxFlySpeed` _charactermovement)) _charactermovement)
  (`/Engine/EditorBlueprintResources/StandardMacros.DoOnce` false :!label _label
    (:`Completed`
      (`GameplayStatics.PlaySoundAtLocation` "/Game/Audio/SFX/slip.slip" (`self.K2_GetActorLocation` _asplayer) (struct) 1.0 1.0 0.0 null null null)
      (goto _label :!via `Reset`))))

(event `LeavePuddle`
  (`KismetSystemLibrary.Delay` 1.0)
  (bind _asplayer (cast `/Game/Blueprints/Player` (`GameplayStatics.GetPlayerCharacter` 0)))
  (`CharacterMovementComponent.SetMovementMode` (`Character.CharacterMovement` _asplayer) "MOVE_Walking" 0)
  (`KismetSystemLibrary.K2_ClearAndInvalidateTimerHandle` (stale `self.Box.OnComponentBeginOverlap` _returnvalue)))

(fn `UserConstructionScript`)