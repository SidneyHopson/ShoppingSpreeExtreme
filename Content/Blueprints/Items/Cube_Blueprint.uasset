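; Breakable cube item that costs the player money when it shatters from a hard impact.
; A hit breaks it if either it or the other actor moves fast, once the post-spawn delay clears the Spawning flag.
; Break plays a poof effect and squish sound, then deducts Price from the player's Money.
; It calls Lose on the player if Money falls below MoneyNeeded, otherwise it destroys itself.
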(event `self.ReceiveBeginPlay`
  (`KismetSystemLibrary.Delay` 5.0)
  (set `self.Spawning` false))

(event `self.ReceiveHit`
  (params (MyComp :type "PrimitiveComponent Object Reference") (Other :type "Actor Object Reference") (OtherComp :type "PrimitiveComponent Object Reference") (bSelfMoved :type Boolean) (HitLocation :type "Vector Structure") (HitNormal :type "Vector Structure") (NormalImpulse :type "Vector Structure") (Hit :type "HitResult Structure (by ref)"))
  (if (and (or (> (`KismetMathLibrary.VSize` (`self.GetVelocity` Other)) 300.0) (> (`KismetMathLibrary.VSize` (`self.GetVelocity`)) 300.0)) (not (`self.Spawning`)))
    (`self.Break`)))

(fn `Break`
  (bind _returnvalue (`self.K2_GetActorLocation`))
  (`GameplayStatics.SpawnEmitterAtLocation` "/Game/StarterContent/Particles/Poof.Poof" _returnvalue)
  (`GameplayStatics.PlaySoundAtLocation` "/Game/Audio/SFX/Squish.Squish" _returnvalue (struct) 0.5 1.0 0.0 null null null)
  (bind _asplayer (cast `/Game/Blueprints/Player` (`GameplayStatics.GetPlayerCharacter` 0)))
  (bind _output_get (set `/Game/Blueprints/Player.Money` (- (`/Game/Blueprints/Player.Money` _asplayer) (`self.Price`)) _asplayer))
  (if (< _output_get (`/Game/Blueprints/Player.MoneyNeeded` _asplayer))
    (`/Game/Blueprints/Player.Lose` _asplayer)
    (else
      (`self.K2_DestroyActor`))))

(fn `UserConstructionScript`)