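; AI-controlled female teen character that reacts when the player or a shopping cart bumps into it.
; A capsule hit from either one sets the CanSeePlayer blackboard key, so the flag signals contact here.
; A DoOnce gate plays the teen voice cue at the character's location, then clears the key and re-arms itself after a short delay.
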(event `self.CapsuleComponent.OnComponentHit`
  (params (HitComponent :type "PrimitiveComponent Object Reference") (OtherActor :type "Actor Object Reference") (OtherComp :type "PrimitiveComponent Object Reference") (NormalImpulse :type "Vector Structure") (Hit :type "HitResult Structure (by ref)"))
  (bind _returnvalue (`AIBlueprintHelperLibrary.GetBlackboard` null))
  (cast `/Game/Blueprints/Player` OtherActor
    (:`then`
      _)
    (:`CastFailed`
      (cast `/Game/Blueprints/ShoppingCart` OtherActor)))
  (`BlackboardComponent.SetValueAsBool` _returnvalue "CanSeePlayer" true)
  (`/Engine/EditorBlueprintResources/StandardMacros.DoOnce` false :!label _label
    (:`Completed`
      (`GameplayStatics.PlaySoundAtLocation` "/Game/Audio/TeenGirl/TeenGirl_Cue.TeenGirl_Cue" (`self.K2_GetActorLocation`) (struct) 1.0 1.0 0.0 null null null)
      (`KismetSystemLibrary.Delay` 2.0)
      (`BlackboardComponent.SetValueAsBool` _returnvalue "CanSeePlayer" false)
      (goto _label :!via `Reset`))))

(fn `UserConstructionScript`
  (`parent.UserConstructionScript`))