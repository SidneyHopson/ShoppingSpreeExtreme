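; NPC_AI is an AI controller that starts NPC behavior and seeds it with patrol settings.
; On BeginPlay it runs the BT_NPC behavior tree and caches the controlled pawn as a BP_NPCBase.
; It then copies the looping flag and wait time from that pawn's PatrolPath into the blackboard, along with an initial forward Direction.
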(event `self.ReceiveBeginPlay`
  (bind _returnvalue (`AIBlueprintHelperLibrary.GetBlackboard` null))
  (`self.RunBehaviorTree` "/Game/Blueprints/AI/BT_NPC.BT_NPC")
  (bind _asbp_npcbase (cast `/Game/Blueprints/AI/BP_NPCBase` (`self.K2_GetPawn`)))
  (bind _output_get (set `self.MyPawn` _asbp_npcbase))
  (`BlackboardComponent.SetValueAsBool` (`AIBlueprintHelperLibrary.GetBlackboard` null) "PathLooping" (`/Game/Blueprints/AI/PatrolPath.isLooping` (`/Game/Blueprints/AI/BP_NPCBase.PatrolPath` _output_get)))
  (`BlackboardComponent.SetValueAsInt` _returnvalue "Direction" 1)
  (`BlackboardComponent.SetValueAsFloat` _returnvalue "WaitTime" (`/Game/Blueprints/AI/PatrolPath.WaitTime` (`/Game/Blueprints/AI/BP_NPCBase.PatrolPath` (`self.MyPawn`)))))

(fn `UserConstructionScript`)