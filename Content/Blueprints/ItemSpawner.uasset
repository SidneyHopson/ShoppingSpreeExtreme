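; One-shot spawner actor that places three copies of a single grocery item class in the level.
; On BeginPlay it picks a random class from fifteen hardcoded products when ItemToSpawn is unset.
; It spawns that class at the location and rotation of three spawn-point components, adjusting for collision but always spawning.
; It then destroys itself after a short delay; SetScale and the construction script are empty.
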(event `self.ReceiveBeginPlay`
  (if (not (`KismetSystemLibrary.IsValidClass` (`self.ItemToSpawn`)))
    (`self.Set Item to Spawn`))
  (`self.SpawnItems`)
  (`KismetSystemLibrary.Delay` 0.5)
  (`self.K2_DestroyActor`))

(fn `Set Item to Spawn`
  (switch `int` (`KismetMathLibrary.RandomIntegerInRange` 0 14)
    (:`0`
      (set `self.ItemToSpawn` "/Game/Blueprints/Items/6Pack_of_Soda.6Pack_of_Soda_C"))
    (:`1`
      (set `self.ItemToSpawn` "/Game/Blueprints/Items/6Pack_of_Soda1.6Pack_of_Soda1_C"))
    (:`2`
      (set `self.ItemToSpawn` "/Game/Blueprints/Items/6Pack_of_Soda2.6Pack_of_Soda2_C"))
    (:`3`
      (set `self.ItemToSpawn` "/Game/Blueprints/Items/6Pack_of_Soda3.6Pack_of_Soda3_C"))
    (:`4`
      (set `self.ItemToSpawn` "/Game/Blueprints/Items/6Pack_of_Soda4.6Pack_of_Soda4_C"))
    (:`5`
      (set `self.ItemToSpawn` "/Game/Blueprints/Items/apple_pie.apple_pie_C"))
    (:`6`
      (set `self.ItemToSpawn` "/Game/Blueprints/Items/Bottle_of_Oil.Bottle_of_Oil_C"))
    (:`7`
      (set `self.ItemToSpawn` "/Game/Blueprints/Items/Bread.Bread_C"))
    (:`8`
      (set `self.ItemToSpawn` "/Game/Blueprints/Items/Cerial.Cerial_C"))
    (:`9`
      (set `self.ItemToSpawn` "/Game/Blueprints/Items/Ham.Ham_C"))
    (:`10`
      (set `self.ItemToSpawn` "/Game/Blueprints/Items/lable_Package.lable_Package_C"))
    (:`11`
      (set `self.ItemToSpawn` "/Game/Blueprints/Items/labledBag.labledBag_C"))
    (:`12`
      (set `self.ItemToSpawn` "/Game/Blueprints/Items/Milk.Milk_C"))
    (:`13`
      (set `self.ItemToSpawn` "/Game/Blueprints/Items/Penut_Butter.Penut_Butter_C"))
    (:`14`
      (set `self.ItemToSpawn` "/Game/Blueprints/Items/Soda.Soda_C"))))

(fn `SetScale`)

(fn `SpawnItems`
  (bind (_returnvalue_location _returnvalue_rotation) (`KismetMathLibrary.BreakTransform` (`SceneComponent.K2_GetComponentToWorld` (`self.Item3Spawn`))))
  (bind (_returnvalue_location_2 _returnvalue_rotation_2) (`KismetMathLibrary.BreakTransform` (`SceneComponent.K2_GetComponentToWorld` (`self.Item1Spawn`))))
  (bind (_returnvalue_location_3 _returnvalue_rotation_3) (`KismetMathLibrary.BreakTransform` (`SceneComponent.K2_GetComponentToWorld` (`self.Item2Spawn`))))
  (`|SpawnActorFromClass` (`self.ItemToSpawn`) (`KismetMathLibrary.MakeTransform` _returnvalue_location_2 _returnvalue_rotation_2) "AdjustIfPossibleButAlwaysSpawn" "OverrideRootScale" null null)
  (`|SpawnActorFromClass` (`self.ItemToSpawn`) (`KismetMathLibrary.MakeTransform` _returnvalue_location_3 _returnvalue_rotation_3) "AdjustIfPossibleButAlwaysSpawn" "OverrideRootScale" null null)
  (`|SpawnActorFromClass` (`self.ItemToSpawn`) (`KismetMathLibrary.MakeTransform` _returnvalue_location _returnvalue_rotation) "AdjustIfPossibleButAlwaysSpawn" "OverrideRootScale" null null))

(fn `UserConstructionScript`)